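; Base NPC Blueprint that lets a character start a dialogue with the player.
; InitiateDialogue checks that the NPC's speaker component and a DialogueSpeakerComponent on player pawn 0 are both valid.
; It then starts the NPC's owned dialogue with both components as speakers and Resume enabled.
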(event EventInitiateDialogue
  (bind _bpc_speakercomponent (Variables|Default|GetBPC_SpeakerComponent))
  (if (and (Utilities|IsValid (Variables|Default|GetBPC_SpeakerComponent)) (Utilities|IsValid (Actor|GetComponentbyClass (Game|Player|GetPlayerPawn 0) "/Script/DialogueTreeRuntime.DialogueSpeakerComponent")))
    (Class|DialogueSpeakerComponent|StartDialogue _bpc_speakercomponent (Class|DialogueSpeakerComponent|GetOwnedDialogue _bpc_speakercomponent) (Utilities|Array|MakeArray (Variables|Default|GetBPC_SpeakerComponent) (Actor|GetComponentbyClass (Game|Player|GetPlayerPawn 0) "/Script/DialogueTreeRuntime.DialogueSpeakerComponent")) true)))

(fn ConstructionScript)
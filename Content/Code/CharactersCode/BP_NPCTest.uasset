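; BP_NPCTest is a test NPC Blueprint for trying out dialogue participant hooks.
; Its OnDialogueStarted event only prints a debug message saying the test dialogue has started.
; The dialogue participant functions are unimplemented stubs: both eligibility checks return false, participant state is Disabled, and the other getters and the path save do nothing.
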(event OnDialogueStarted(BP_NPCTest)
  (Development|PrintString "the test dialogue has been started"))

(fn ConstructionScript)

(fn CanParticipateinDialogue
  (return false))

(fn CanStartDialogue
  (return false))

(fn GetAudioComponent
  (return 0))

(fn GetDefaultParticipantState
  (return "EDPS_Disabled"))

(fn GetDialogueGraph
  (return 0))

(fn GetOwningActor
  (return 0))

(fn GetParticipantState
  (return "EDPS_Disabled"))

(fn GetParticipantTag
  (return ""))

(fn GetSavedStartingNode
  (return 0))

(fn GetTraversedPath
  (return 0))

(fn SaveTraversedPath
  (return 0))
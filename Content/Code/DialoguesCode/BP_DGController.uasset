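; Dialogue controller that creates and drives the on-screen dialogue widget, using settings from the dialogue manager subsystem.
; On BeginPlay it caches those settings and adds the widget, quitting the game if it lacks BI_SimpleDialogueDisplay.
; Open, close, speech and option events are forwarded through that interface, with input mode and cursor switched for dialogue and restored on close.
; A missing speaker prints its name and quits the game.
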(event Custom|Initialize
  ;[1 1 1] Initialize: Add Widget of Specified Type To Viewport
  (Dialogue|CacheSettings)
  (bind _returnvalue (UserInterface|CreateWidget (Variables|Dialogue|GetWidgetType) (Game|GetPlayerController 0)))
  (if (Utilities|DoesObjectImplementInterface _returnvalue "/DialogueTree/DisplayWidgets/BI_SimpleDialogueDisplay.BI_SimpleDialogueDisplay_C")
    (bind _output_get (Variables|Dialogue|SetDialogueWidget _returnvalue))
    (UserInterface|Viewport|AddtoViewport _output_get (Variables|Dialogue|GetWidgetZOrder))
    (Widget|SetVisibility _output_get "Visible")
    (Class|BISimpleDialogueDisplay|SetController(Message) _output_get self)
    (else
      (Game|QuitGame 0 "Quit" false))))

(event EventHandleMissingSpeaker
  (params (MissingName :type Name%20%28by%20ref%29 :default "None"))
  ;[1 1 1] Missing Speaker
  (Development|PrintString (Utilities|String|ToString(Name) MissingName))
  (Game|QuitGame (Game|GetPlayerController 0) "Quit" false))

(event EventCloseDisplay
  (bind _dialoguewidget (Variables|Dialogue|GetDialogueWidget))
  ;[1 1 1] Close the Widget
  (Utilities|IsValid _dialoguewidget
    (:Is%20Valid
      (Widget|SetVisibility _dialoguewidget "Collapsed")
      (Dialogue|RevertInputMode)
      (if (Utilities|DoesObjectImplementInterface (Variables|Dialogue|GetDialogueWidget) "/DialogueTree/DisplayWidgets/BI_SimpleDialogueDisplay.BI_SimpleDialogueDisplay_C")
        (Class|BISimpleDialogueDisplay|OnClose(Message) (Variables|Dialogue|GetDialogueWidget))))))

(event EventOpenDisplay
  ;[1 1 1] Open the Widget
  (Utilities|IsValid (Variables|Dialogue|GetDialogueWidget)
    (:Is%20Valid
      (Widget|SetVisibility (Variables|Dialogue|GetDialogueWidget) "SelfHitTestInvisible")
      (Dialogue|SetInputModeforDialogue)
      (if (Utilities|DoesObjectImplementInterface (Variables|Dialogue|GetDialogueWidget) "/DialogueTree/DisplayWidgets/BI_SimpleDialogueDisplay.BI_SimpleDialogueDisplay_C")
        (Class|BISimpleDialogueDisplay|OnOpen(Message) (Variables|Dialogue|GetDialogueWidget))))))

(event EventBeginPlay
  ;[1 1 1] Sets up the controller at start
  (CallFunction|Initialize))

(event EventDisplayOptions
  (params (InOptions :type Array%20of%20Speech%20Details%20Structures))
  (bind _dialoguewidget (Variables|Dialogue|GetDialogueWidget))
  ;[1 1 1] Display Options
  (Utilities|IsValid _dialoguewidget
    (:Is%20Valid
      (Class|BISimpleDialogueDisplay|DisplayOptions(Message) _dialoguewidget InOptions))))

(event EventDisplaySpeech
  (params (InSpeechDetails :type Speech%20Details%20Structure) (InSpeaker :type Dialogue%20Speaker%20Component%20Object%20Reference))
  (bind _dialoguewidget (Variables|Dialogue|GetDialogueWidget))
  ;[1 1 1] Display Speech
  (Utilities|IsValid _dialoguewidget
    (:Is%20Valid
      (Class|BISimpleDialogueDisplay|DisplaySpeech(Message) _dialoguewidget InSpeechDetails InSpeaker))))

(fn ConstructionScript)

(fn CanOpenDisplay
  (bind _dialoguewidget (Variables|Dialogue|GetDialogueWidget))
  (return (and (Utilities|IsValid _dialoguewidget) (Utilities|DoesObjectImplementInterface _dialoguewidget "/DialogueTree/DisplayWidgets/BI_SimpleDialogueDisplay.BI_SimpleDialogueDisplay_C"))))

(fn RevertInputMode
  (bind _defaultinputmode (Variables|Dialogue|GetDefaultInputMode))
  (bind (_inputmode _flushinput _hidecursorduringcapture) (Utilities|Struct|BreakDLGInputModeSettings _defaultinputmode))
  (LocalVariables|SetLocalPlayerController (Game|GetPlayerController 0))
  ;[1 1 1] Retrieve Mouse Lock Mode - Translate to Desired Enum from Accessible Counterpart
  (switch Utilities|FlowControl|Switch|SwitchonEDLGMouseLockMode (.MouseLockMode (Utilities|Struct|BreakDLGInputModeSettings (Variables|Dialogue|GetDefaultInputMode)))
    (:DoNotLock
      (LocalVariables|SetLocalMouseLockMode "DoNotLock"))
    (:LockOnCapture
      (LocalVariables|SetLocalMouseLockMode "LockOnCapture"))
    (:LockAlways
      (LocalVariables|SetLocalMouseLockMode "LockAlways"))
    (:LockInFullscreen
      (LocalVariables|SetLocalMouseLockMode "LockInFullscreen")))
  ;[1 1 1] Determine Target Input Mode
  (switch Utilities|FlowControl|Switch|SwitchonEDLGInputMode (.InputMode (Utilities|Struct|BreakDLGInputModeSettings (Variables|Dialogue|GetDefaultInputMode)))
    (:GameOnly
      ;[1 1 1] Game Only
      (Input|SetInputModeGameOnly (LocalVariables|GetLocalPlayerController) (.FlushInput (Utilities|Struct|BreakDLGInputModeSettings (Variables|Dialogue|GetDefaultInputMode))))
      (Class|GameplayStatics|SetViewportMouseCaptureMode "CapturePermanently_IncludingInitialMouseDown"))
    (:GameAndUI
      ;[1 1 1] Game and UI
      (Input|SetInputModeGameandUI (LocalVariables|GetLocalPlayerController) 0 (LocalVariables|GetLocalMouseLockMode) _hidecursorduringcapture _flushinput))
    (:UIOnly
      ;[1 1 1] UI Only
      (Input|SetInputModeUIOnly (LocalVariables|GetLocalPlayerController) 0 (LocalVariables|GetLocalMouseLockMode) (.FlushInput (Utilities|Struct|BreakDLGInputModeSettings (Variables|Dialogue|GetDefaultInputMode))))))
  ;[1 1 1] Revert Mouse Cursor Visibility
  (Variables|/Script/Engine.PlayerController|SetbShowMouseCursor (LocalVariables|GetLocalPlayerController) (Variables|Dialogue|GetCachedShowMouseCursor)))

(fn SetInputModeforDialogue
  (LocalVariables|SetLocalPlayerController (Game|GetPlayerController 0))
  (if (Variables|Dialogue|GetAllowGameInputInDialogue)
    ;[1 1 1] Game Input + UI allowed
    (Input|SetInputModeGameandUI (LocalVariables|GetLocalPlayerController) (Variables|Dialogue|GetDialogueWidget) "DoNotLock" false true)
    (else
      ;[1 1 1] Only UI Input Allowed
      (Input|SetInputModeUIOnly (LocalVariables|GetLocalPlayerController) (Variables|Dialogue|GetDialogueWidget) "DoNotLock" true)))
  ;[1 1 1] Cache Previous Cursor Visibility
  (Variables|Dialogue|SetCachedShowMouseCursor (Variables|/Script/Engine.PlayerController|GetbShowMouseCursor (LocalVariables|GetLocalPlayerController)))
  ;[1 1 1] Ensure Mouse Cursor is Visible
  (Variables|/Script/Engine.PlayerController|SetbShowMouseCursor (LocalVariables|GetLocalPlayerController) true))

(fn CacheSettings
  (bind _returnvalue (Subsystems|GetDialogueManagerSubsystem))
  (bind _returnvalue_2 (Class|DialogueManagerSubsystem|GetSettings _returnvalue))
  (Variables|Dialogue|SetWidgetZOrder (Variables|/Script/DialogueTreeRuntime.DialogueSettings|GetWidgetZOrder _returnvalue_2))
  (Variables|Dialogue|SetDefaultInputMode (Variables|/Script/DialogueTreeRuntime.DialogueSettings|GetDefaultInputMode _returnvalue_2))
  (Variables|Dialogue|SetAllowGameInputInDialogue (Variables|/Script/DialogueTreeRuntime.DialogueSettings|GetAllowGameInputInDialogue _returnvalue_2))
  ;[1 1 1] Only set widget type if the override type is valid - else keep default
  (bind _returnvalue_3 (Utilities|LoadClassAssetBlocking (Variables|/Script/DialogueTreeRuntime.DialogueSettings|GetDialogueWidgetType _returnvalue_2)))
  (bind _asuser_widget (Utilities|Casting|CastToUserWidgetClass _returnvalue_3))
  (Variables|Dialogue|SetWidgetType _asuser_widget))

(fn GetDialogueWidget
  (return (Variables|Dialogue|GetDialogueWidget)))
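; Dialogue manager component for the player controller that selects dialogue nodes from the current dialogue data table.
; PlayDialogueNode searches rows by ID, stores the match and fires the controller's play-node delegate.
; Rows requiring a cocktail check the player character and raise a status notification if it is missing, but still count as found.
; It also rebroadcasts detail button clicks through a delegate, while SetFirstRow is an empty stub.
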(event Custom|PlayDialogueNode
  (params (RowID :type Integer))
  (bind (_browfound _foundrowdata) (CallFunction|FindDGRowbyID RowID))
  (if _browfound
    (Variables|Default|SetDT%20values%20holder _foundrowdata)
    (bind _asbp_player_controller (Utilities|Casting|CastToBP_PlayerController (Components|GetOwner)))
    (Default|CallDelegatePlayNode _asbp_player_controller)))

(event Custom|SetFirstRow)

(fn FindDGRowbyID
  (params (SearchID :type Integer))
  (bind _currentdialoguetable (Variables|Default|GetCurrentDialogueTable))
  (bind _outrownames (DataTable|GetDataTableRowNames _currentdialoguetable))
  (for _array_element _outrownames
    (bind _returnvalue (Utilities|GetDataTableRow _currentdialoguetable _array_element)
      (:then
        (if (== (.ID (Utilities|Struct|BreakST_Dialogue _returnvalue)) SearchID)
          (if (not (.bcocktailrequired (.CocktailMiniGame (Utilities|Struct|BreakST_Dialogue _returnvalue))))
            _
            (else
              (bind _asbp_character (Utilities|Casting|CastToBP_Character (Game|Player|GetPlayerPawn 0)))
              (if (Variables|/Game/Code/Basics/BP_Character.BP_Character_C|GetbCocktailPresent _asbp_character)
                _
                (else
                  (Default|CallCocktailStatusNotify (Variables|/Game/Code/Basics/BP_Character.BP_Character_C|GetbCocktailPresent _asbp_character))
                  (return true _returnvalue (Variables|/Game/Code/Basics/BP_Character.BP_Character_C|GetbCocktailPresent _asbp_character))))))
          (return true _returnvalue false)))))
  (return false "" false))

(fn BroadcastDetailClicked
  (params (ButtonRowName :type Name) (DetailObjRef :type WBP%20Details%20Button%20Object%20Reference))
  (Default|CallDelegateDetailButtonClicked ButtonRowName DetailObjRef)
  (return))
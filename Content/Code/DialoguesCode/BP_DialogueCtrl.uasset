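; BP_DialogueCtrl is the dialogue controller that passes speech lines and player options to the on-screen UI.
; On BeginPlay it finds the top-level WBP_MainScene widget, caches it and registers itself as that widget's controller.
; Its DisplaySpeech and DisplayOptions events forward their data to the widget after a validity check, with leftover debug prints in the speech path.
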(event EventBeginPlay
  (bind _foundwidgets (Widget|GetAllWidgetsOfClass "/Game/Code/Widgets/MainScene/WBP_MainScene.WBP_MainScene_C" true))
  (for _array_element _foundwidgets
    (Variables|Default|SetMainSceneWidget _array_element))
  (Default|SetController (Variables|Default|GetMainSceneWidget) self))

(event EventDisplaySpeech
  (params (InSpeechDetails :type Speech%20Details%20Structure) (InSpeaker :type Dialogue%20Speaker%20Component%20Object%20Reference))
  (Utilities|IsValid (Variables|Default|GetMainSceneWidget)
    (:Is%20Valid
      (Default|DisplaySpeech (Variables|Default|GetMainSceneWidget) InSpeechDetails InSpeaker)
      (Development|PrintString "kurw?"))
    (:Is%20Not%20Valid
      (Development|PrintString "kurwaa"))))

(event EventDisplayOptions
  (params (InOptions :type Array%20of%20Speech%20Details%20Structures))
  (Utilities|IsValid (Variables|Default|GetMainSceneWidget)
    (:Is%20Valid
      (Default|DisplayOptions (Variables|Default|GetMainSceneWidget) InOptions))))

(fn ConstructionScript
  (|CallParentFunction))